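; Sphere player Blueprint that places and colors itself for one of two players, based on PlayerInt.
; Its construction script registers SphereBody through SetBodySphereMeshComp.
; On BeginPlay it moves to the PlayerStart tagged "player" plus PlayerInt, then applies that player's material.
; Hitting another SpherePlayer_BP zeroes its own body's physics linear velocity.
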(event EventBeginPlay
  (CallFunction|SpawnFunction)
  (CallFunction|SetColor))

(event Collision|EventHit
  (params (MyComp :type Primitive%20Component%20Object%20Reference) (Other :type Actor%20Object%20Reference) (OtherComp :type Primitive%20Component%20Object%20Reference) (bSelfMoved :type Boolean) (HitLocation :type Vector :default "0, 0, 0") (HitNormal :type Vector :default "0, 0, 0") (NormalImpulse :type Vector :default "0, 0, 0") (Hit :type Hit%20Result%20Structure%20%28by%20ref%29))
  (Utilities|Casting|CastToSpherePlayer_BP Other)
  (Class|PrimitiveComponent|SetAllPhysicsLinearVelocity (Variables|Default|GetSphere%20Body) "0, 0, 0" false))

(fn ConstructionScript
  (Class|SpherePlayer|SetBodySphereMeshComp (Variables|Default|GetSphere%20Body)))

(fn SpawnFunction
  (bind _outactors (Actor|GetAllActorsOfClass "/Script/Engine.PlayerStart"))
  (for _array_element _outactors
    (bind _asplayer_start (Utilities|Casting|CastToPlayerStart _array_element))
    (if (Utilities|Enum|Equal(Enum) (Utilities|String|ToString(Name) (Variables|/Script/Engine.PlayerStart|GetPlayerStartTag _asplayer_start)) (Utilities|String|Append "player" (Utilities|String|ToString(Integer) (Variables|Default|GetPlayerInt))))
      (bind _output_get (Variables|Default|SetSpawnLocation (Transformation|GetActorTransform _asplayer_start)))
      (Transformation|SetActorTransform _output_get))))

(fn SetColor
  (bind _sphere_body (Variables|Default|GetSphere%20Body))
  (switch int (Variables|Default|GetPlayerInt)
    (:0
      (Rendering|Material|SetMaterial _sphere_body 0 "/Game/Material/Player1_Mat.Player1_Mat"))
    (:1
      (Rendering|Material|SetMaterial _sphere_body 0 "/Game/Material/Player2_Mat.Player2_Mat"))))