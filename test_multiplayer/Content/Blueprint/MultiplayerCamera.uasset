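; Shared camera actor that frames two local players by tracking their midpoint and zooming with their separation.
; After a brief delay on BeginPlay it caches both player pawns and stores starting camera position values, which the graph never reads.
; Each Tick it computes player distance and center, interpolates the spring arm length toward the clamped distance, and moves a Box component to the midpoint.
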(event Custom|Set%20distance%20between%20players
  ;[1 1 1] Set distance beetween players
  (Variables|Default|SetDistBetween2Player (Transformation|GetDistanceTo (Variables|Default|GetPlayer1) (Variables|Default|GetPlayer2))))

(event Custom|CameraZoom
  (bind _springarm (Variables|Default|GetSpringArm))
  ;[1 1 1] Camera zoom
  (Variables|/Script/Engine.SpringArmComponent|SetTargetArmLength _springarm (Math|Interpolation|FInterpTo (Variables|/Script/Engine.SpringArmComponent|GetTargetArmLength _springarm) (Math|Float|Clamp(Float) (Variables|Default|GetDistBetween2Player) 1.5e+03 5e+03) (Variables|Default|GetDelta) 5e+01)))

(event Custom|Move%20Camera
  ;[1 1 1] Set the box location
  (Transformation|SetWorldLocation (Variables|Default|GetBox) (Variables|Default|GetCenter%20Position) false false))

(event Custom|Set%20Center%20Point
  ;[1 1 1] Set center point between our players
  (Variables|Default|SetCenter%20Position (/ (+ (Transformation|GetActorLocation (Variables|Default|GetPlayer1)) (Transformation|GetActorLocation (Variables|Default|GetPlayer2))) 2)))

(event EventBeginPlay
  (bind _springarm (Variables|Default|GetSpringArm))
  (bind _returnvalue (Transformation|GetWorldLocation _springarm))
  (Utilities|FlowControl|Delay 0.005)
  (Utilities|FlowControl|Sequence
    (:then_0
      (Variables|Default|SetPlayer1 (Game|Player|GetPlayerPawn 0))
      (Variables|Default|SetPlayer2 (Game|Player|GetPlayerPawn 1)))
    (:then_1
      (Variables|Default|SetCamXPos (.x _returnvalue))
      (Variables|Default|SetCamYPos (.y _returnvalue))
      (Variables|Default|SetCamStartPos (Math|Vector|MakeVector 0.0 0.0 (.z (Transformation|GetActorLocation)))))))

(event EventTick
  (params (DeltaSeconds :type Float%20%28single-precision%29))
  (Variables|Default|SetDelta DeltaSeconds)
  (CallFunction|SetDistanceBetweenPlayers)
  (CallFunction|SetCenterPoint)
  (CallFunction|CameraZoom)
  (CallFunction|MoveCamera))

(fn ConstructionScript)