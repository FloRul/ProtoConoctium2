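; Game mode that sets up a two-player local multiplayer session with a shared camera.
; On BeginPlay it creates a second local player, then spawns a SpherePlayer_BP at a fixed point for each controller, passes in its player index and possesses it.
; It caches the first MultiplayerCamera found in the level and, after a brief delay, makes it player 0's view target.
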(event Custom|Find%20Multiplayer%20Camera
  (bind _outactors (Actor|GetAllActorsOfClass "/Game/Blueprint/MultiplayerCamera.MultiplayerCamera_C"))
  (Variables|Default|SetMain%20Camera (Utilities|Array|Get(acopy) _outactors)))

(event EventBeginPlay
  (CallFunction|SpawnPlayers)
  (CallFunction|FindMultiplayerCamera)
  (Utilities|FlowControl|Delay 0.02)
  (Game|Player|SetViewTargetwithBlend (Game|GetPlayerController 0) (Variables|Default|GetMain%20Camera) 0.0 "VTBlend_Linear" 0.0 false))

(fn ConstructionScript)

(fn SpawnPlayers
  (for _index (range 1 1)
    (Class|GameplayStatics|CreatePlayer _index))
  (for _index_2 (range 0 1)
    (bind _returnvalue (Game|SpawnActorfromClass "/Game/Blueprint/SpherePlayer_BP.SpherePlayer_BP_C" (Math|Transform|MakeTransform "0.000000, 0,200.000000") "Undefined" 0 _index_2 0))
    (Pawn|Possess (Game|GetPlayerController _index_2) _returnvalue)))