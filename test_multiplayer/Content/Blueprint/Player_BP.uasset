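; Player Blueprint that places and colors itself on BeginPlay according to its PlayerInt index.
; SpawnFunction searches all PlayerStart actors for a tag matching "player" plus the index and moves the actor to that start's transform.
; SetColor then gives the Sphere the Player 1 or Player 2 material for index 0 or 1.
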(event EventBeginPlay
  (CallFunction|SpawnFunction)
  (CallFunction|SetColor))

(event Collision|EventActorBeginOverlap
  (params (OtherActor :type Actor%20Object%20Reference)))

(event EventTick
  (params (DeltaSeconds :type Float%20%28single-precision%29)))

(fn ConstructionScript)

(fn SpawnFunction
  (bind _outactors (Actor|GetAllActorsOfClass "/Script/Engine.PlayerStart"))
  (for _array_element _outactors
    (bind _asplayer_start (Utilities|Casting|CastToPlayerStart _array_element))
    (if (Utilities|Enum|Equal(Enum) (Utilities|String|ToString(Name) (Variables|/Script/Engine.PlayerStart|GetPlayerStartTag _asplayer_start)) (Utilities|String|Append "player" (Utilities|String|ToString(Integer) (Variables|Default|GetPlayerInt))))
      (bind _output_get (Variables|Default|SetSpawnLocation (Transformation|GetActorTransform _asplayer_start)))
      (Transformation|SetActorTransform _output_get))))

(fn SetColor
  (bind _sphere (Variables|Default|GetSphere))
  (switch int (Variables|Default|GetPlayerInt)
    (:0
      (Rendering|Material|SetMaterial _sphere 0 "/Game/Material/Player1_Mat.Player1_Mat"))
    (:1
      (Rendering|Material|SetMaterial _sphere 0 "/Game/Material/Player2_Mat.Player2_Mat"))))